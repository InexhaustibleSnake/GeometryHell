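; Player character Blueprint that handles death, pausing, camera zoom and a post-process effect.
; The HealthComponent's death event clears all widgets, shows the game-over screen, pauses the game and switches to UI-only input.
; The post-process shows while Q is held from a standstill and also follows the TimeStopped event.
; Holding R narrows the camera's field of view, and the Pause action calls CallPauseEvent.
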(event `self.ReceiveBeginPlay`
  (add `HealthComponent.OnDeath` (`self.HealthComponent`) (delegate `OnDeath_Event_0`)))

(event `OnDeath_Event_0`
  (bind _returnvalue (`GameplayStatics.GetPlayerController` 0))
  (`WidgetLayoutLibrary.RemoveAllWidgets`)
  (bind _returnvalue_2 (`|CreateWidget` "/Game/MainContent/UI/WBP_GameOver.WBP_GameOver_C"))
  (`UserWidget.AddToViewport` _returnvalue_2 0)
  (`GameplayStatics.SetGamePaused` true)
  (`WidgetBlueprintLibrary.SetInputMode_UIOnlyEx` _returnvalue null "LockAlways")
  (set `PlayerController.bShowMouseCursor` true _returnvalue))

(event `TimeStopped`
  (params (WasTimeStopped :type Boolean))
  (if WasTimeStopped
    (`SceneComponent.SetVisibility` (`self.PostProcess`) true false)
    (else
      (`SceneComponent.SetVisibility` (`self.PostProcess`) false false))))

(event `Key|Q`
  (params (Key :type "Key Structure"))
  (:`Pressed`
    (if (== (`KismetMathLibrary.VSize` (`self.GetVelocity`)) 0.0)
      (`SceneComponent.SetVisibility` (`self.PostProcess`) true false)))
  (:`Released`
    (`SceneComponent.SetVisibility` (`self.PostProcess`) false false)))

(event `Key|R`
  (params (Key :type "Key Structure"))
  (bind _maincamera (`self.MainCamera`))
  (:`Pressed`
    (`CameraComponent.SetFieldOfView` _maincamera 30.0))
  (:`Released`
    (`CameraComponent.SetFieldOfView` _maincamera 90.0)))

(event `InputAction|Pause`
  (params (Key :type "Key Structure"))
  (:`Pressed`
    (`self.PauseEvent`)))

(fn `UserConstructionScript`)