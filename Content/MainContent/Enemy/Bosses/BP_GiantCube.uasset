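; BP_GiantCube is a giant cube boss enemy that manages its on-screen widget and damage feedback.
; On BeginPlay it adds WBP_GiantCube to the viewport and binds its damage and destroyed events.
; Any damage briefly swaps the CannonCube material to a hurt material, then restores it.
; On destruction it removes the first WBP_GiantCube found by a class search, rather than using a stored reference.
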(event `self.ReceiveBeginPlay`
  (add `Actor.OnTakeAnyDamage` (delegate `OnTakeAnyDamage_Event_0`))
  (bind _returnvalue (`|CreateWidget` "/Game/MainContent/Enemy/Bosses/WBP_GiantCube.WBP_GiantCube_C"))
  (`UserWidget.AddToViewport` _returnvalue 0)
  (add `Actor.OnDestroyed` (delegate `OnDestroyed_Event_0`)))

(event `OnTakeAnyDamage_Event_0`
  (params (DamagedActor :type "Actor Object Reference") (Damage :type "Float (double-precision)") (DamageType :type "DamageType Object Reference") (InstigatedBy :type "Controller Object Reference") (DamageCauser :type "Actor Object Reference"))
  (`PrimitiveComponent.SetMaterial` (`self.CannonCube`) 0 "/Game/MainContent/Enemy/Bosses/M_GiantCubeHurt.M_GiantCubeHurt")
  (`KismetSystemLibrary.Delay` 0.2)
  (`PrimitiveComponent.SetMaterial` (`self.CannonCube`) 0 "/Game/MainContent/Enemy/Bosses/M_GiantCubeCannon.M_GiantCubeCannon"))

(event `OnDestroyed_Event_0`
  (params (DestroyedActor :type "Actor Object Reference"))
  (bind _foundwidgets (`WidgetBlueprintLibrary.GetAllWidgetsOfClass` "/Game/MainContent/Enemy/Bosses/WBP_GiantCube.WBP_GiantCube_C"))
  (`Widget.RemoveFromParent` (`|GetArrayItem` _foundwidgets)))

(fn `UserConstructionScript`)