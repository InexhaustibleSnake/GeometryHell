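; BP_FinalBoss is the final boss enemy, handling its on-screen widget and relaying its time-stop ability to the player.
; On BeginPlay it caches the player as BP_MainCharacter and binds its TimeStop dispatcher to call TimeStopped on that character with the active state.
; It also adds a WBP_FinalBoss widget to the viewport and, when destroyed, removes the first such widget it finds by class.
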(event `self.ReceiveBeginPlay`
  (bind _asbp_main_character (cast `/Game/MainContent/Player/BP_MainCharacter` (`GameplayStatics.GetPlayerCharacter` 0)))
  (set `self.Player` _asbp_main_character)
  (add `self.TimeStop` (delegate `TimeStop_Event_0`))
  (bind _returnvalue (`|CreateWidget` "/Game/MainContent/Enemy/Bosses/FinalBoss/WBP_FinalBoss.WBP_FinalBoss_C"))
  (`UserWidget.AddToViewport` _returnvalue 0)
  (add `Actor.OnDestroyed` (delegate `OnDestroyed_Event_0`)))

(event `TimeStop_Event_0` :!signature `self.TimeStop`
  (params (IsActive :type Boolean))
  (`/Game/MainContent/Player/BP_MainCharacter.TimeStopped` (`self.Player`) IsActive))

(event `OnDestroyed_Event_0`
  (params (DestroyedActor :type "Actor Object Reference"))
  (bind _foundwidgets (`WidgetBlueprintLibrary.GetAllWidgetsOfClass` "/Game/MainContent/Enemy/Bosses/FinalBoss/WBP_FinalBoss.WBP_FinalBoss_C"))
  (`Widget.RemoveFromParent` (`|GetArrayItem` _foundwidgets)))

(fn `UserConstructionScript`)