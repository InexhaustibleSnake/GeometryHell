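; BP_Sphere is a damageable piece of the final boss encounter that hurts the boss when it is destroyed.
; On BeginPlay it binds to its own damage event, which briefly swaps the CannonCube material to a hurt material, then restores the green health material.
; When destroyed, it applies fixed damage to the first BP_FinalBoss found in the level.
; This graph contains no health tracking or destroy logic.
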(event `self.ReceiveBeginPlay`
  (add `Actor.OnTakeAnyDamage` (delegate `OnTakeAnyDamage_Event_0`)))

(event `OnTakeAnyDamage_Event_0`
  (params (DamagedActor :type "Actor Object Reference") (Damage :type "Float (double-precision)") (DamageType :type "DamageType Object Reference") (InstigatedBy :type "Controller Object Reference") (DamageCauser :type "Actor Object Reference"))
  (`PrimitiveComponent.SetMaterial` (`self.CannonCube`) 0 "/Game/MainContent/Enemy/M_Hurt.M_Hurt")
  (`KismetSystemLibrary.Delay` 0.2)
  (`PrimitiveComponent.SetMaterial` (`self.CannonCube`) 0 "/Game/MainContent/Pickups/M_GreenHealth.M_GreenHealth"))

(event `self.ReceiveDestroyed`
  (bind _outactors (`GameplayStatics.GetAllActorsOfClass` "/Game/MainContent/Enemy/Bosses/FinalBoss/BP_FinalBoss.BP_FinalBoss_C"))
  (`GameplayStatics.ApplyDamage` (`|GetArrayItem` _outactors) 100.0))

(fn `UserConstructionScript`)