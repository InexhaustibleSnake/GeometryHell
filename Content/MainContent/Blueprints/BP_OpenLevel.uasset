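; BP_OpenLevel is a level-transition actor that opens the level named in LevelName when the player character overlaps it.
; On BeginPlay it caches the player, the game instance and the save object loaded from slot Save1.
; After the open call, it unlocks Second Level or Third Level in both game instance and save, then writes the slot.
; A matching fourth-level unlock exists but is never run.
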(event `self.ReceiveBeginPlay`
  (bind _asbp_main_character (cast `/Game/MainContent/Player/BP_MainCharacter` (`GameplayStatics.GetPlayerCharacter` 0)))
  (set `self.Player` _asbp_main_character)
  (bind _asbp_base_game_instance (cast `/Game/MainContent/Logic/BP_BaseGameInstance` (`GameplayStatics.GetGameInstance`)))
  (set `self.GameInstance` _asbp_base_game_instance)
  (bind _returnvalue (`GameplayStatics.LoadGameFromSlot` "Save1"))
  (bind _asbp_save_1 (cast `/Game/MainContent/Logic/Saves/BP_Save1` _returnvalue))
  (set `self.SavedGame` _asbp_save_1))

(event `self.ReceiveActorBeginOverlap`
  (params (OtherActor :type "Actor Object Reference"))
  (bind _levelname (`self.LevelName`))
  (bind _savedgame (`self.SavedGame`))
  (bind _savedgame_2 (`self.SavedGame`))
  (if (== OtherActor (`self.Player`))
    (`GameplayStatics.OpenLevel` _levelname)
    (switch `string` (`KismetStringLibrary.Conv_NameToString` _levelname)
      (:`SecondLevel`
        (set `/Game/MainContent/Logic/BP_BaseGameInstance.LevelTwoUnlocked` true (`self.GameInstance`))
        (set `/Game/MainContent/Logic/Saves/BP_Save1.SecondLevelUnlocked` true _savedgame)
        (`GameplayStatics.SaveGameToSlot` _savedgame "Save1"))
      (:`ThirdLevel`
        (set `/Game/MainContent/Logic/BP_BaseGameInstance.LevelThreeUnlocked` true (`self.GameInstance`))
        (set `/Game/MainContent/Logic/Saves/BP_Save1.ThirdLevelUnlocked` true _savedgame_2)
        (`GameplayStatics.SaveGameToSlot` _savedgame_2 "Save1")))))

(fn `UserConstructionScript`)