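; Moving platform that stays still until the player character first enters its trigger box, then starts moving.
; The construction script builds four relative InterpToMovement control points from its location variables and applies the configured duration.
; BeginPlay caches the player and halts the movement component.
; A DoOnce on the box overlap restarts that movement, so later overlaps have no effect.
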(event `self.ReceiveBeginPlay`
  (bind _asbp_main_character (cast `/Game/MainContent/Player/BP_MainCharacter` (`GameplayStatics.GetPlayerCharacter` 0)))
  (set `self.Player` _asbp_main_character)
  (`MovementComponent.StopMovementImmediately` (`self.InterpToMovement`)))

(event `self.Box.OnComponentBeginOverlap`
  (params (OverlappedComponent :type "PrimitiveComponent Object Reference") (OtherActor :type "Actor Object Reference") (OtherComp :type "PrimitiveComponent Object Reference") (OtherBodyIndex :type Integer) (bFromSweep :type Boolean) (SweepResult :type "HitResult Structure (by ref)"))
  (if (== OtherActor (`self.Player`))
    (`/Engine/EditorBlueprintResources/StandardMacros.DoOnce` false
      (:`Completed`
        (`InterpToMovementComponent.RestartMovement` (`self.InterpToMovement`) 1.0)))))

(fn `UserConstructionScript`
  (bind _interptomovement (`self.InterpToMovement`))
  (set `InterpToMovementComponent.ControlPoints` (`|MakeArray` (make `InterpControlPoint` (`self.Location1`)) (make `InterpControlPoint` (`self.Location2`)) (make `InterpControlPoint` (`self.Location3`)) (make `InterpControlPoint` (`self.Location4`))) _interptomovement)
  (set `InterpToMovementComponent.Duration` (`self.Duration`) _interptomovement))