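; BP_KillBox is a hidden hazard that damages actors and reveals itself when the player comes near.
; The Cube mesh starts invisible and applies BaseDamage to any actor that begins overlapping it.
; A separate Box trigger shows the Cube with a 2D click sound when the cached BP_MainCharacter enters, and hides it again on exit.
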(event `self.ReceiveBeginPlay`
  (`SceneComponent.SetVisibility` (`self.Cube`) false false)
  (bind _asbp_main_character (cast `/Game/MainContent/Player/BP_MainCharacter` (`GameplayStatics.GetPlayerCharacter` 0)))
  (set `self.Player` _asbp_main_character))

(event `self.Cube.OnComponentBeginOverlap`
  (params (OverlappedComponent :type "PrimitiveComponent Object Reference") (OtherActor :type "Actor Object Reference") (OtherComp :type "PrimitiveComponent Object Reference") (OtherBodyIndex :type Integer) (bFromSweep :type Boolean) (SweepResult :type "HitResult Structure (by ref)"))
  (`GameplayStatics.ApplyDamage` OtherActor (`self.Base Damage`)))

(event `self.Box.OnComponentBeginOverlap`
  (params (OverlappedComponent :type "PrimitiveComponent Object Reference") (OtherActor :type "Actor Object Reference") (OtherComp :type "PrimitiveComponent Object Reference") (OtherBodyIndex :type Integer) (bFromSweep :type Boolean) (SweepResult :type "HitResult Structure (by ref)"))
  (if (== OtherActor (`self.Player`))
    (`SceneComponent.SetVisibility` (`self.Cube`) true false)
    (`GameplayStatics.PlaySound2D` "/Game/MainContent/Sound/Interface/SC_Click.SC_Click" 1.0 1.0 0.0 null null)))

(event `self.Box.OnComponentEndOverlap`
  (params (OverlappedComponent :type "PrimitiveComponent Object Reference") (OtherActor :type "Actor Object Reference") (OtherComp :type "PrimitiveComponent Object Reference") (OtherBodyIndex :type Integer))
  (if (== OtherActor (`self.Player`))
    (`SceneComponent.SetVisibility` (`self.Cube`) false false)))

(fn `UserConstructionScript`)