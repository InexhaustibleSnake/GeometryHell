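; BP_SlideDoor is a door that slides upward when the player character enters its trigger box, then closes itself.
; On BeginPlay it caches player 0's pawn as BP_MainCharacter, so only that actor triggers the box.
; The OpenDoor timeline drives a lerp on the door mesh's relative location, and its Finished pin waits briefly before reversing the timeline to lower the door.
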(event `self.ReceiveBeginPlay`
  (bind _asbp_main_character (cast `/Game/MainContent/Player/BP_MainCharacter` (`GameplayStatics.GetPlayerCharacter` 0)))
  (set `self.Player` _asbp_main_character))

(event `self.Box.OnComponentBeginOverlap`
  (params (OverlappedComponent :type "PrimitiveComponent Object Reference") (OtherActor :type "Actor Object Reference") (OtherComp :type "PrimitiveComponent Object Reference") (OtherBodyIndex :type Integer) (bFromSweep :type Boolean) (SweepResult :type "HitResult Structure (by ref)"))
  (if (== OtherActor (`self.Player`))
    (bind (_direction _newtrack_0) (`Timeline|OpenDoor` :!via `PlayFromStart` :!label _label)
      (:`Update`
        (`SceneComponent.K2_SetRelativeLocation` (`self.SM_Door`) (`KismetMathLibrary.VLerp` (0.0 0.0 0.0) (0.0 0.0 250.0) _newtrack_0) false false))
      (:`Finished`
        (`KismetSystemLibrary.Delay` 2.0)
        (goto _label :!via `Reverse`)))))

(fn `UserConstructionScript`)