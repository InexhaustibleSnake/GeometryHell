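; BP_StartPlayOst is a trigger volume that starts a 2D sound, presumably soundtrack music, when the player enters it.
; On BeginPlay it caches the player character as BP_MainCharacter.
; The Box overlap spawns the sound only for that cached player and sets WasTriggered, so it fires once per instance.
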(event `self.ReceiveBeginPlay`
  (bind _asbp_main_character (cast `/Game/MainContent/Player/BP_MainCharacter` (`GameplayStatics.GetPlayerCharacter` 0)))
  (set `self.Player` _asbp_main_character))

(event `self.Box.OnComponentBeginOverlap`
  (params (OverlappedComponent :type "PrimitiveComponent Object Reference") (OtherActor :type "Actor Object Reference") (OtherComp :type "PrimitiveComponent Object Reference") (OtherBodyIndex :type Integer) (bFromSweep :type Boolean) (SweepResult :type "HitResult Structure (by ref)"))
  (if (and (== OtherActor (`self.Player`)) (not (`self.WasTriggered`)))
    (`GameplayStatics.SpawnSound2D` (`self.Sound`) 1.0 1.0 0.0 null)
    (set `self.WasTriggered` true)))

(fn `UserConstructionScript`)