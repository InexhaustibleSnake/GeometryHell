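; BP_FinalBossProjectile is a final boss projectile that homes in on the player character.
; From BeginPlay it loops every 0.2 seconds, enabling homing and setting the ProjectileMovementComponent's target from FindPlayer.
; FindPlayer takes the first BP_MainCharacter and returns its scene component only when it is nearer than the stored ClosesDistance, which then shrinks to that distance.
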(event `GoToTarget`
  (bind _projectilemovementcomponent (`self.ProjectileMovementComponent`))
  (bind _playertarget (`self.FindPlayer`))
  (set `ProjectileMovementComponent.HomingTargetComponent` _playertarget _projectilemovementcomponent)
  (set `ProjectileMovementComponent.bIsHomingProjectile` true _projectilemovementcomponent))

(event `self.ReceiveBeginPlay`
  (`self.GoToTarget` :!label _label)
  (`KismetSystemLibrary.Delay` 0.2)
  (goto _label))

(fn `FindPlayer`
  (returns (PlayerTarget :type "SceneComponent Object Reference"))
  (bind _outactors (`GameplayStatics.GetAllActorsOfClass` "/Game/MainContent/Player/BP_MainCharacter.BP_MainCharacter_C"))
  (bind _output (`|GetArrayItem` _outactors))
  (bind _output_get (set `self.Player` _output))
  (`/Engine/EditorBlueprintResources/StandardMacros.IsValid` _output_get
    (:`Is Valid`
      (bind _returnvalue (`KismetMathLibrary.VSize` (- (`self.K2_GetActorLocation` _output) (`self.K2_GetActorLocation`))))
      (if (< _returnvalue (`self.ClosesDistance`))
        (set `self.ClosesDistance` _returnvalue)
        (return (`self.GetComponentByClass` (`self.Player`) "/Script/Engine.SceneComponent"))))))

(fn `UserConstructionScript`)